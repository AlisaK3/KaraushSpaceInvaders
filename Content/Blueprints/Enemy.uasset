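; Space Invaders-style enemy that restarts the level when it overlaps the PlayerShip.
; Two alternating timelines move it sideways and step it along negative X, flipping direction after each sweep.
; After a delay, a looping timer with a randomized per-enemy interval gives a chance to spawn an EnemyBullet at the Cube.
; DestroyEnemy removes it and increments the player's kill count, granting a capped extra life at the eighth kill.
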(event Custom|Destroy%20Enemy
  (Actor|DestroyActor)
  (bind _asplayer_ship (Utilities|Casting|CastToPlayerShip (Game|Player|GetPlayerPawn 0)))
  (bind _output_get (Variables|/Game/Blueprints/PlayerShip.PlayerShip_C|SetHowMuchKills _asplayer_ship (+ (Variables|/Game/Blueprints/PlayerShip.PlayerShip_C|GetHowMuchKills _asplayer_ship) 1)))
  (if (== _output_get 8)
    (if (< (Variables|/Game/Blueprints/PlayerShip.PlayerShip_C|GetLives _asplayer_ship) 3)
      (bind _output_get_2 (Variables|/Game/Blueprints/PlayerShip.PlayerShip_C|SetLives _asplayer_ship (+ (Variables|/Game/Blueprints/PlayerShip.PlayerShip_C|GetLives _asplayer_ship) 1)))
      (Development|PrintString (Utilities|String|ToString(Integer) _output_get_2) true true "(R=0.937480,G=1.000000,B=0.000000,A=1.000000)"))))

(event Custom|Bullet%20spawn
  (if (> (Math|Random|RandomFloatinRange 0.0 1.0) 0.75)
    (Game|SpawnActorfromClass "/Game/Blueprints/EnemyBullet.EnemyBullet_C" (Math|Conversions|ToTransform(Vector) (Transformation|GetWorldLocation (Variables|Default|GetCube))) "Undefined" 0 0)))

(event EventBeginPlay
  (Utilities|FlowControl|Sequence
    (:then_0
      (Timeline|Timeline_0 Play
        (:Update
          (if (Variables|Default|GetMoveRight)
            (Transformation|AddActorWorldOffset "0,1.000000, 0")
            (else
              (Transformation|AddActorWorldOffset "0,-1.000000, 0"))))
        (:Finished
          (Variables|Default|SetMoveRight (not (Variables|Default|GetMoveRight)))
          (Timeline|Timeline_1 PlayFromStart
            (:Update
              (Transformation|AddActorWorldOffset "-1.000000,0.000000, 0"))
            (:Finished
              (if (Variables|Default|GetMoveRight)
                (Timeline|Timeline_0 PlayFromStart)
                (else
                  (Timeline|Timeline_0 ReverseFromEnd))))))))
    (:then_1
      (Utilities|FlowControl|Delay 2.0)
      (Utilities|Time|SetTimerbyEvent (delegate Custom|Bullet%20spawn) (Math|Random|RandomFloatinRange 2.0 5.0) true)
      (if (> (Math|Random|RandomFloatinRange 0.0 1.0) 0.75)
        (Game|SpawnActorfromClass "/Game/Blueprints/EnemyBullet.EnemyBullet_C" (Math|Conversions|ToTransform(Vector) (Transformation|GetWorldLocation (Variables|Default|GetCube))) "Undefined" 0 0)))))

(event Collision|EventActorBeginOverlap
  (params (OtherActor :type Actor%20Object%20Reference))
  (bind _asplayer_ship (Utilities|Casting|CastToPlayerShip OtherActor))
  (Default|RestartLevel _asplayer_ship))

(fn ConstructionScript)