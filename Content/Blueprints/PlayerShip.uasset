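; Player ship that slides sideways, fires bullets and handles game over, in what looks like an arcade shooter.
; Input flags drive a fixed, frame-rate-dependent Y step on Tick without sweep, with left taking priority.
; Shooting spawns a bullet at the Gun and clears BullDissap, blocking further shots until something outside this file resets it.
; Restartlevel disables input, plays a game-over sound, then reloads the level after a delay.
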(event Custom|Restart%20level
  (Input|DisableInput 0)
  (Utilities|FlowControl|Sequence
    (:then_0
      (Audio|PlaySoundatLocation "/Game/522670__baltiyar13__game-over-8-bit.522670__baltiyar13__game-over-8-bit" "0, 0, 0" "0, 0, 0" 1.0 1.0 0.0 0 0 0))
    (:then_1
      (Utilities|FlowControl|Delay 3.0)
      (Game|OpenLevel(byName) "Untitled"))))

(event EventBeginPlay
  (bind _output_get (Variables|Default|SetHowMuchKills 0))
  (Variables|Default|SetMaxLives _output_get))

(event EventTick
  (params (DeltaSeconds :type Float%20%28single-precision%29))
  (if (Variables|Default|GetMoveLeft)
    (Transformation|SetActorLocation (+ (Transformation|GetActorLocation) "0,-10.000000, 0") false false)
    (elif (Variables|Default|GetMoveRight)
      (Transformation|SetActorLocation (+ (Transformation|GetActorLocation) "0,10.000000, 0") false false))))

(event Input|ActionEvents|InputActionMoveLeft
  (params (Key :type Key%20Structure :default "None"))
  (:Pressed
    (Variables|Default|SetMoveLeft true))
  (:Released
    (Variables|Default|SetMoveLeft false)))

(event Input|ActionEvents|InputActionMoveRight
  (params (Key :type Key%20Structure :default "None"))
  (:Pressed
    (Variables|Default|SetMoveRight true))
  (:Released
    (Variables|Default|SetMoveRight false)))

(event Input|ActionEvents|InputActionShoot
  (params (Key :type Key%20Structure :default "None"))
  (:Pressed
    (if (Variables|Default|GetBullDissap)
      (Game|SpawnActorfromClass "/Game/Blueprints/PlayerBullet.PlayerBullet_C" (Math|Conversions|ToTransform(Vector) (Transformation|GetWorldLocation (Variables|Default|Getgun))) "Undefined" 0 0)
      (Audio|PlaySoundatLocation "/Game/344310__musiclegends__laser-shoot.344310__musiclegends__laser-shoot" "0, 0, 0" "0, 0, 0" 1.0 1.0 0.0 0 0 0)
      (Variables|Default|SetBullDissap false))))

(fn ConstructionScript)