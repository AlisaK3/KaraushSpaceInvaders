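; PlayerBullet is the player's projectile, reacting when its Sphere component begins overlapping another actor.
; Casts sort the hit: an Enemy gets DestroyEnemy and the bullet destroys itself, while a DestrWall is destroyed and an EndForBullets actor is left intact.
; All three cases set BullDissap on the PlayerShip pawn; only the Enemy case destroys the bullet here.
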(event OnComponentBeginOverlap(Sphere)
  (params (OverlappedComponent :type Primitive%20Component%20Object%20Reference) (OtherActor :type Actor%20Object%20Reference) (OtherComp :type Primitive%20Component%20Object%20Reference) (OtherBodyIndex :type Integer) (bFromSweep :type Boolean) (SweepResult :type Hit%20Result%20Structure%20%28by%20ref%29))
  (bind _asenemy (Utilities|Casting|CastToEnemy OtherActor)
    (:then
      (Default|DestroyEnemy _asenemy)
      (Actor|DestroyActor)
      (bind _asplayer_ship (Utilities|Casting|CastToPlayerShip (Game|Player|GetPlayerPawn 0)))
      (Variables|/Game/Blueprints/PlayerShip.PlayerShip_C|SetBullDissap _asplayer_ship true))
    (:CastFailed
      (bind _asdestr_wall (Utilities|Casting|CastToDestrWall OtherActor)
        (:then
          (Actor|DestroyActor _asdestr_wall)
          (bind _asplayer_ship_2 (Utilities|Casting|CastToPlayerShip (Game|Player|GetPlayerPawn 0)))
          (Variables|/Game/Blueprints/PlayerShip.PlayerShip_C|SetBullDissap _asplayer_ship_2 true))
        (:CastFailed
          (Utilities|Casting|CastToEndForBullets OtherActor)
          (bind _asplayer_ship_3 (Utilities|Casting|CastToPlayerShip (Game|Player|GetPlayerPawn 0)))
          (Variables|/Game/Blueprints/PlayerShip.PlayerShip_C|SetBullDissap _asplayer_ship_3 true))))))

(event EventBeginPlay)

(event Collision|EventActorBeginOverlap
  (params (OtherActor :type Actor%20Object%20Reference)))

(event EventTick
  (params (DeltaSeconds :type Float%20%28single-precision%29)))

(fn ConstructionScript)